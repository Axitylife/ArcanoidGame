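; BP_Ball is a ball actor that travels in a straight line and bounces off whatever blocks it.
; Each Tick on the authority, it performs a swept world offset along DirectionBall, scaled by Speed and delta time, in X and Y only.
; On a blocking hit, DirectionBall is mirrored around the surface normal, giving simple reflection bounces without physics simulation.
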(event `self.ReceiveTick`
  (params (DeltaSeconds :type "Float (single-precision)"))
  (bind (_returnvalue_x _returnvalue_y) (`KismetMathLibrary.BreakVector` (* (`self.Direction ball`) (* DeltaSeconds (`self.Speed`)))))
  (`/Engine/EditorBlueprintResources/ActorMacros.Switch Has Authority`
    (:`Authority`
      (bind _sweephitresult (`self.K2_AddActorWorldOffset` (`KismetMathLibrary.MakeVector` _returnvalue_x _returnvalue_y) true)))
    (:`Remote`
      _))
  (bind (_bblockinghit _binitialoverlap _time _distance _location _impactpoint _normal) (`GameplayStatics.BreakHitResult` _sweephitresult))
  (if _bblockinghit
    (set `self.Direction ball` (`KismetMathLibrary.GetReflectionVector` (`self.Direction ball`) _normal))))

(fn `UserConstructionScript`)