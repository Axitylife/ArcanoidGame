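; BP_Block is a destructible block that takes a random number of hits to break and may drop a bonus.
; At BeginPlay the authority rolls the hit count, which indexes the cube's material.
; Each cube hit lowers the count and updates the material; a hit at ZeroHit triggers OnLastHit.
; OnLastHit runs Bonus, which occasionally spawns BP_BonusBallx2 at the cube's location, then destroys the block.
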(event `Set destroy hit`)

(event `OnLastHit`
  ;[1 1 1] Last hit event
  (`self.Bonus`)
  (`self.K2_DestroyActor`))

(event `self.ReceiveBeginPlay`
  ;[1 1 1] Set material and random hit for box
  (`/Engine/EditorBlueprintResources/ActorMacros.Switch Has Authority`
    (:`Authority`
      (set `self.Destroy Hit` (`KismetMathLibrary.RandomIntegerInRange` 0 2)))
    (:`Remote`
      _))
  (`PrimitiveComponent.SetMaterial` (`self.Cube`) 0 (`|GetArrayItem` (`self.Color Material`) (`self.Destroy Hit`))))

(event `self.Cube.OnComponentHit`
  (params (HitComponent :type "PrimitiveComponent Object Reference") (OtherActor :type "Actor Object Reference") (OtherComp :type "PrimitiveComponent Object Reference") (NormalImpulse :type "Vector Structure") (Hit :type "HitResult Structure (by ref)"))
  ;[1 1 1] IF hit == 0 destroyed; else set material;
  (`/Engine/EditorBlueprintResources/ActorMacros.Switch Has Authority`
    (:`Authority`
      _)
    (:`Remote`
      _))
  (if (== (`self.Destroy Hit`) (`self.ZeroHit`))
    (`self.OnLastHit`)
    (else
      (bind _result (`/Engine/EditorBlueprintResources/StandardMacros.DecrementInt` (`self.Destroy Hit`))
        (:`  `
          (set `self.Destroy Hit` _result)
          (`PrimitiveComponent.SetMaterial` (`self.Cube`) 0 (`|GetArrayItem` (`self.Color Material`) (`self.Destroy Hit`))))))))

(event `Bonus`
  ;[1 1 1] Bonus
  (if (<= (`KismetMathLibrary.RandomFloatInRange` 0.0 1.0) 0.1)
    (`|SpawnActorFromClass` "/Game/Blueprints/BP_BonusBallx2.BP_BonusBallx2_C" (`KismetMathLibrary.MakeTransform` (`SceneComponent.K2_GetComponentLocation` (`self.Cube`))) "AlwaysSpawn" "OverrideRootScale" null null)))

(fn `UserConstructionScript`)