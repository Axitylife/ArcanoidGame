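; BP_BonusBallx2 is a moving bonus actor that doubles the balls in play when it hits something.
; Each Tick it makes a swept move along Direction at Speed.
; On any blocking hit, whatever the object, it spawns a half-scale BP_Ball at each existing ball's sphere with a fixed diagonal DirectionBall.
; It calls DestroyActor inside that loop, so it is only destroyed if a ball exists.
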(event `self.ReceiveTick`
  (params (DeltaSeconds :type "Float (single-precision)"))
  (bind _returnvalue_x (`KismetMathLibrary.BreakVector` (* (`self.Direction`) (* DeltaSeconds (`self.Speed`)))))
  ;[1 1 1] Comment
  (bind _sweephitresult (`self.K2_AddActorWorldOffset` (`KismetMathLibrary.MakeVector` _returnvalue_x) true))
  (if (`GameplayStatics.BreakHitResult` _sweephitresult)
    (bind _outactors (`GameplayStatics.GetAllActorsOfClass` "/Game/Blueprints/BP_Ball.BP_Ball_C"))
    (for _array_element _outactors
      (bind _returnvalue (`|SpawnActorFromClass` "/Game/Blueprints/BP_Ball.BP_Ball_C" (`KismetMathLibrary.MakeTransform` (`SceneComponent.K2_GetComponentLocation` (`/Game/Blueprints/BP_Ball.Sphere` _array_element)) (struct) (0.5 0.5 0.5)) "Undefined" "OverrideRootScale" null null))
      (set `/Game/Blueprints/BP_Ball.Direction ball` (1.0 -1.0 0.0) _returnvalue)
      (`self.K2_DestroyActor`))))

(fn `UserConstructionScript`)